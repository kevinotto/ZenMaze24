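; MenuGroundBP is an actor, apparently the tiltable maze ground shown in the menu, that rotates in response to mouse movement.
; Mouse X and Y axis input accumulates into roll and pitch values, each clamped to a symmetric 45-degree limit.
; Every tick applies those values as the world rotation of the root component, keeping yaw at zero.
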(event `self.ReceiveTick`
  (params (DeltaSeconds :type "Float (single-precision)"))
  ;[1 1 1] Updates rotation values of maze object
  (`SceneComponent.K2_SetWorldRotation` (`self.DefaultSceneRoot`) (`KismetMathLibrary.MakeRotator` (`self.RotX`) (`self.RotY`)) false false))

(event `InputAxisKey|MouseX`
  (params (AxisValue :type "Float (single-precision)"))
  ;[1 1 1] Mouse X rotation
  (set `self.RotX` (`KismetMathLibrary.FClamp` (+ AxisValue (`self.RotX`)) -45.0 45.0)))

(event `InputAxisKey|MouseY`
  (params (AxisValue :type "Float (single-precision)"))
  ;[1 1 1] Mouse Y rotation
  (set `self.RotY` (`KismetMathLibrary.FClamp` (+ AxisValue (`self.RotY`)) -45.0 45.0)))

(fn `UserConstructionScript`)